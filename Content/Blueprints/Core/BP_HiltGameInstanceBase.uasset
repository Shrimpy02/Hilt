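; Base Game Instance that owns the game's save object and handles saving and loading it to a named slot.
; Loading an existing slot or saving can run sync or async, then calls a loaded or saved notification.
; Save requests gather every actor implementing BPI_Saveble into BP_SaveGame before writing to disk.
; Load requests restore data per requester from the held save object without rereading the slot.
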(event `LoadGame`
  (params (Async :type Boolean))
  (bind _savegameslotname (`self.SaveGameSlotName`))
  ;[1 1 1] LoadGAme
  (bind _returnvalue (`GameplayStatics.DoesSaveGameExist` (`self.SaveGameSlotName`)))
  (if _returnvalue
    (if Async
      (bind _savegame (`AsyncActionHandleSaveGame.AsyncLoadGameFromSlot` _savegameslotname)
        (:`Completed`
          (bind _asbp_save_game (cast `/Game/Blueprints/Core/BP_SaveGame` _savegame))
          (bind _output_get (set `self.SaveGameRef` _asbp_save_game))
          (`self.GameLoaded` _output_get)))
      (else
        (bind _returnvalue_2 (`GameplayStatics.LoadGameFromSlot` _savegameslotname))
        (bind _asbp_save_game_2 (cast `/Game/Blueprints/Core/BP_SaveGame` _returnvalue_2))
        (bind _output_get_2 (set `self.SaveGameRef` _asbp_save_game_2))
        (`self.GameLoaded` _output_get_2)))))

(event `CreateSaveGame`
  ;[1 1 1] Create Save game
  (bind _returnvalue (`GameplayStatics.CreateSaveGameObject` "/Game/Blueprints/Core/BP_SaveGame.BP_SaveGame_C"))
  (set `self.SaveGameRef` _returnvalue))

(event `SaveGame`
  (params (Async :type Boolean))
  (bind _savegameref (`self.SaveGameRef`))
  (bind _savegameref_2 (`self.SaveGameRef`))
  (bind _savegameslotname (`self.SaveGameSlotName`))
  ;[1 1 1] SaveGame
  (if Async
    (`AsyncActionHandleSaveGame.AsyncSaveGameToSlot` _savegameref null _savegameslotname
      (:`Completed`
        (`self.GameSaved` _savegameref_2)))
    (else
      (`GameplayStatics.SaveGameToSlot` _savegameref _savegameslotname)
      (`self.GameSaved` _savegameref_2))))

(event `/Game/Blueprints/Core/BPI_Presistance.RequestSave`
  (params (Async :type Boolean))
  ;[1 1 1] Request Save
  (bind _outactors (`GameplayStatics.GetAllActorsWithInterface` "/Game/Blueprints/Core/BPI_Saveble.BPI_Saveble_C"))
  (`/Game/Blueprints/Core/BP_SaveGame.SaveAllData` (`self.SaveGameRef`) _outactors)
  (`self.SaveGame` Async))

(event `/Game/Blueprints/Core/BPI_Presistance.RequestLoad`
  (params (Requester :type "Object Object Reference"))
  (`/Game/Blueprints/Core/BP_SaveGame.LoadDataForRequestor` (`self.SaveGameRef`) Requester))