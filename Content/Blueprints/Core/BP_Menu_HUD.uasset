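; Menu HUD that creates a WBP_MenuStack on BeginPlay and opens the main menu on it.
; Events push screens such as options, level select, credits, security cam and loading onto that stack, with loading also pausing the game.
; Pause instead uses ToggleWidget, which collapses other listed widgets and switches input mode and cursor between game and UI.
; Other events toggle stack visibility and reset the player overlay on restart.
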(event `self.ReceiveBeginPlay`
  (`|ExecutionSequence`
    (:`then_0`
      ;[1 1 1] Refrences
      (set `self.Player Controller` (`self.GetOwningPlayerController`))
      (bind _asbp_hilt_game_instance_base (cast `/Game/Blueprints/Core/BP_HiltGameInstanceBase` (`GameplayStatics.GetGameInstance`)))
      (set `self.Game Instance` _asbp_hilt_game_instance_base)
      (bind _asbp_hilt_game_mode_base (cast `/Game/Blueprints/Core/BP_HiltGameModeBase` (`GameplayStatics.GetGameMode`)))
      (set `self.GameMode` _asbp_hilt_game_mode_base)
      (bind _asbp_player_character (cast `/Game/Blueprints/Player/BP_PlayerCharacter` (`GameplayStatics.GetPlayerCharacter` 0)))
      (set `self.PlayerCharacter` _asbp_player_character))
    (:`then_1`
      ;[1 1 1] Set up layout
      (bind _returnvalue (`|CreateWidget` "/Game/Blueprints/Widget/WBP_MenuStack.WBP_MenuStack_C" (`self.Player Controller`)))
      (bind _output_get (set `self.LayoutMenu` _returnvalue))
      (`UserWidget.AddToViewport` _output_get 0)
      (`/Game/Blueprints/Widget/WBP_MenuStack.Push Widget` _output_get "/Game/Blueprints/Widget/WBP_CommonMainMenu.WBP_CommonMainMenu_C"))))

(event `ToggleSecurity Cam`
  ;[1 1 1] Toggle Securty Cam Widget
  (`/Game/Blueprints/Widget/WBP_MenuStack.Push Widget` (`self.LayoutMenu`) "/Game/Blueprints/Widget/WBP_SecurityCam.WBP_SecurityCam_C"))

(event `TogglePause`
  ;[1 1 1] Toggle pause
  (`GameplayStatics.SetGamePaused` true)
  (`self.Toggle_widget` (`self.PauseRef`)))

(event `ToggleCoreMenu`
  ;[1 1 1] Toggle menu
  (`/Game/Blueprints/Widget/WBP_MenuStack.Push Widget` (`self.LayoutMenu`) "/Game/Blueprints/Widget/WBP_CommonMainMenu.WBP_CommonMainMenu_C"))

(event `ToggleHUDVisibility`
  (bind _layoutmenu (`self.LayoutMenu`))
  ;[1 1 1] Toggle Hud visibility
  (if (== (`Widget.Visibility` _layoutmenu) 1)
    (set `Widget.Visibility` "Visible" _layoutmenu)
    (else
      (set `Widget.Visibility` "Collapsed" _layoutmenu))))

(event `ToggleOptions`
  ;[1 1 1] Toggle options
  (`/Game/Blueprints/Widget/WBP_MenuStack.Push Widget` (`self.LayoutMenu`) "/Game/Blueprints/Widget/WBP_CommonOptions.WBP_CommonOptions_C"))

(event `ToggleLevelSelect`
  ;[1 1 1] Toggle level select
  (`/Game/Blueprints/Widget/WBP_MenuStack.Push Widget` (`self.LayoutMenu`) "/Game/Blueprints/Widget/WBP_CommonLevelSelect.WBP_CommonLevelSelect_C"))

(event `Hud Restart`
  ;[1 1 1] Respawn Player Event
  (bind _aswbp_player_overlay (cast `/Game/Blueprints/Widget/OldWidgets/WBP_PlayerOverlay` (`self.CoreHUDRef`)))
  (`/Game/Blueprints/Widget/OldWidgets/WBP_PlayerOverlay.Reset On Restart` _aswbp_player_overlay))

(event `ToggleLoadingScreen`
  ;[1 1 1] Toggle level select
  (`GameplayStatics.SetGamePaused` true)
  (`/Game/Blueprints/Widget/WBP_MenuStack.Push Widget` (`self.LayoutMenu`) "/Game/Blueprints/Widget/WBP_CommonLoadingScreen.WBP_CommonLoadingScreen_C"))

(event `ToggleCredits`
  ;[1 1 1] Credits
  (`/Game/Blueprints/Widget/WBP_MenuStack.Push Widget` (`self.LayoutMenu`) "/Game/Blueprints/Widget/WBP_CommonCredits.WBP_CommonCredits_C"))

(fn `FocusGame`
  (bind _player_controller (`self.Player Controller`))
  (`Widget.SetVisibility` (`self.Widget to Focus`) "Collapsed")
  (`WidgetBlueprintLibrary.SetInputMode_GameOnly` _player_controller)
  (set `PlayerController.bShowMouseCursor` false _player_controller))

(fn `FocusWidget`
  (bind _player_controller (`self.Player Controller`))
  (`Widget.SetVisibility` (`self.Widget to Focus`) "SelfHitTestInvisible")
  (`WidgetBlueprintLibrary.SetInputMode_UIOnlyEx` _player_controller (`self.Widget to Focus`) "LockOnCapture")
  (set `PlayerController.bShowMouseCursor` true _player_controller))

(fn `Toggle_widget`
  (params (WidgetToFocus :type "UserWidget Object Reference"))
  (`/Engine/EditorBlueprintResources/StandardMacros.IsValid` WidgetToFocus
    (:`Is Valid`
      (set `self.Widget to Focus` WidgetToFocus)
      (for _array_element (`self.GameMenu_WidgetList`)
        (`/Engine/EditorBlueprintResources/StandardMacros.IsValid` _array_element
          (:`Is Valid`
            (if (== (`self.Widget to Focus`) _array_element)
              (if (`Widget.IsVisible` (`self.Widget to Focus`))
                (`self.FocusGame`)
                (else
                  (`self.FocusWidget`)))
              (elif (`Widget.IsVisible` _array_element)
                (`Widget.SetVisibility` _array_element "Collapsed")))))))))

(fn `UserConstructionScript`)