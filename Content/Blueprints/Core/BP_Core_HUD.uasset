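; Core HUD that creates and manages the player overlay, core menu, options, pause, end-level and level-select screens.
; BeginPlay spawns each widget into a shared list and adds them to the viewport.
; Toggle events feed ToggleWidget, which flips the target's visibility, collapses the others and switches input mode and cursor.
; Pause and end-level events also change game pause state, while HudRestart resets the player overlay.
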(event `self.ReceiveBeginPlay`
  (`|ExecutionSequence`
    (:`then_0`
      ;[1 1 1] Refrences
      (set `self.Player Controller` (`self.GetOwningPlayerController`))
      (bind _asbp_hilt_game_instance_base (cast `/Game/Blueprints/Core/BP_HiltGameInstanceBase` (`GameplayStatics.GetGameInstance`)))
      (set `self.Game Instance` _asbp_hilt_game_instance_base))
    (:`then_1`
      ;[1 1 1] Player overlay
      (bind _returnvalue (`|CreateWidget` (`self.CoreHUD`)))
      (bind _output_get (set `self.CoreHUDRef` _returnvalue))
      (`UserWidget.AddToViewport` _returnvalue 0)
      (`KismetArrayLibrary.Array_Add` (`self.GameMenu_WidgetList`) _output_get))
    (:`then_2`
      ;[1 1 1] Game Menu's
      (bind _returnvalue_2 (`|CreateWidget` (`self.CoreMenu`)))
      (bind _output_get_2 (set `self.CoreMenuRef` _returnvalue_2))
      (`KismetArrayLibrary.Array_Add` (`self.GameMenu_WidgetList`) _output_get_2)
      (bind _returnvalue_3 (`|CreateWidget` (`self.Option`)))
      (bind _output_get_3 (set `self.OptionRef` _returnvalue_3))
      (`KismetArrayLibrary.Array_Add` (`self.GameMenu_WidgetList`) _output_get_3)
      (bind _returnvalue_4 (`|CreateWidget` (`self.Pause`)))
      (bind _output_get_4 (set `self.PauseRef` _returnvalue_4))
      (`KismetArrayLibrary.Array_Add` (`self.GameMenu_WidgetList`) _output_get_4)
      (bind _returnvalue_5 (`|CreateWidget` (`self.EndLevel`)))
      (bind _output_get_5 (set `self.EndLevelRef` _returnvalue_5))
      (`KismetArrayLibrary.Array_Add` (`self.GameMenu_WidgetList`) _output_get_5)
      (bind _returnvalue_6 (`|CreateWidget` (`self.LevelSelect`)))
      (bind _output_get_6 (set `self.LevelSelectRef` _returnvalue_6))
      (`KismetArrayLibrary.Array_Add` (`self.GameMenu_WidgetList`) _output_get_6))
    (:`then_3`
      ;[1 1 1] Add to Viewport
      (for _array_element (`self.GameMenu_WidgetList`)
        (`/Engine/EditorBlueprintResources/StandardMacros.IsValid` _array_element
          (:`Is Valid`
            (`UserWidget.AddToViewport` _array_element 0)))))))

(event `ToggleCoreHUD`
  (bind _player_controller (`self.Player Controller`))
  ;[1 1 1] Toggle Hud
  (`self.Toggle_widget` (`self.CoreHUDRef`))
  (`WidgetBlueprintLibrary.SetInputMode_GameOnly` _player_controller true)
  (set `PlayerController.bShowMouseCursor` false _player_controller))

(event `ToggleCoreMenu`
  ;[1 1 1] Toggle menu
  (`self.Toggle_widget` (`self.CoreMenuRef`)))

(event `TogglePause`
  ;[1 1 1] Toggle pause
  (`GameplayStatics.SetGamePaused` true)
  (`self.Toggle_widget` (`self.PauseRef`)))

(event `ToggleOptions`
  (bind _optionref (`self.OptionRef`))
  (bind _player_controller (`self.Player Controller`))
  ;[1 1 1] Toggle options
  (`self.Toggle_widget` _optionref)
  (`WidgetBlueprintLibrary.SetInputMode_UIOnlyEx` _player_controller _optionref)
  (set `PlayerController.bShowMouseCursor` true _player_controller))

(event `ToggleEndLevel`
  ;[1 1 1] Toggle end level
  (`self.Toggle_widget` (`self.EndLevelRef`))
  (if (`GameplayStatics.IsGamePaused`)
    (`GameplayStatics.SetGamePaused` false)
    (else
      (`GameplayStatics.SetGamePaused` true))))

(event `ToggleLevelSelect`
  ;[1 1 1] Toggle level select
  (`self.Toggle_widget` (`self.LevelSelectRef`)))

(event `Hud Restart`
  ;[1 1 1] Respawn Player Event
  (bind _aswbp_player_overlay (cast `/Game/Blueprints/Widget/WBP_PlayerOverlay` (`self.CoreHUDRef`)))
  (`/Game/Blueprints/Widget/WBP_PlayerOverlay.Reset On Restart` _aswbp_player_overlay))

(fn `FocusGame`
  (bind _player_controller (`self.Player Controller`))
  (`Widget.SetVisibility` (`self.Widget to Focus`) "Collapsed")
  (`WidgetBlueprintLibrary.SetInputMode_GameOnly` _player_controller)
  (set `PlayerController.bShowMouseCursor` false _player_controller))

(fn `FocusWidget`
  (bind _player_controller (`self.Player Controller`))
  (`Widget.SetVisibility` (`self.Widget to Focus`) "SelfHitTestInvisible")
  (`WidgetBlueprintLibrary.SetInputMode_UIOnlyEx` _player_controller (`self.Widget to Focus`) "LockOnCapture")
  (set `PlayerController.bShowMouseCursor` true _player_controller))

(fn `Toggle_widget`
  (params (WidgetToFocus :type "UserWidget Object Reference"))
  (`/Engine/EditorBlueprintResources/StandardMacros.IsValid` WidgetToFocus
    (:`Is Valid`
      (set `self.Widget to Focus` WidgetToFocus)
      (for _array_element (`self.GameMenu_WidgetList`)
        (`/Engine/EditorBlueprintResources/StandardMacros.IsValid` _array_element
          (:`Is Valid`
            (if (== (`self.Widget to Focus`) _array_element)
              (if (`Widget.IsVisible` (`self.Widget to Focus`))
                (`self.FocusGame`)
                (else
                  (`self.FocusWidget`)))
              (elif (`Widget.IsVisible` _array_element)
                (`Widget.SetVisibility` _array_element "Collapsed")))))))))

(fn `UserConstructionScript`)