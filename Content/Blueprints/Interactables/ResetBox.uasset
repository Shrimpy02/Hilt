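; ResetBox is an interactable trigger volume that sends the player back to their current spawn point when they enter it.
; BeginPlay caches the BP_PlayerCharacter; on overlap with that player, it gathers all BP_SpawnPoint actors.
; It moves the player to the one whose array index matches the player's PlayerSpawnPointIndex, relying on GetAllActorsOfClass ordering rather than an ID on each spawn point.
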(event `self.ReceiveBeginPlay`
  (bind _asbp_player_character (cast `/Game/Blueprints/Player/BP_PlayerCharacter` (`GameplayStatics.GetPlayerCharacter` 0)))
  (set `self.BP_Player` _asbp_player_character))

(event `self.ResetBox.OnComponentBeginOverlap`
  (params (OverlappedComponent :type "PrimitiveComponent Object Reference") (OtherActor :type "Actor Object Reference") (OtherComp :type "PrimitiveComponent Object Reference") (OtherBodyIndex :type Integer) (bFromSweep :type Boolean) (SweepResult :type "HitResult Structure (by ref)"))
  (if (== (`self.BP_Player`) OtherActor)
    (bind _outactors (`GameplayStatics.GetAllActorsOfClass` "/Game/Blueprints/Interactables/BP_SpawnPoint.BP_SpawnPoint_C"))
    (for (_array_element _array_index) _outactors
      (if (== _array_index (`PlayerCharacter.PlayerSpawnPointIndex` (`self.BP_Player`)))
        (`self.K2_SetActorLocation` (`self.BP_Player`) (`self.K2_GetActorLocation` _array_element) false false)))))

(fn `UserConstructionScript`)