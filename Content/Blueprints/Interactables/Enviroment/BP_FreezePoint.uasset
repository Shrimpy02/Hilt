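; BP_FreezePoint is an environment interactable that triggers freeze-related functions on the player character.
; On BeginPlay it finds BP_PlayerCharacter actors and caches the last one as its player reference.
; A box overlap by an actor tagged Player calls KillFreeze on that cached player and destroys the point.
; Any hit on the mesh calls CoolHook on the same player, regardless of what struck it.
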(event `self.ReceiveBeginPlay`
  (bind _outactors (`GameplayStatics.GetAllActorsOfClass` "/Game/Blueprints/Player/BP_PlayerCharacter.BP_PlayerCharacter_C"))
  (for _array_element _outactors
    (set `self.As BP Player Character` _array_element)))

(event `self.Box.OnComponentBeginOverlap`
  (params (OverlappedComponent :type "PrimitiveComponent Object Reference") (OtherActor :type "Actor Object Reference") (OtherComp :type "PrimitiveComponent Object Reference") (OtherBodyIndex :type Integer) (bFromSweep :type Boolean) (SweepResult :type "HitResult Structure (by ref)"))
  (if (`self.ActorHasTag` OtherActor "Player")
    (`/Game/Blueprints/Player/BP_PlayerCharacter.KillFreeze` (`self.As BP Player Character`))
    (`self.K2_DestroyActor`)))

(event `self.Mesh.OnComponentHit`
  (params (HitComponent :type "PrimitiveComponent Object Reference") (OtherActor :type "Actor Object Reference") (OtherComp :type "PrimitiveComponent Object Reference") (NormalImpulse :type "Vector Structure") (Hit :type "HitResult Structure (by ref)"))
  (`/Game/Blueprints/Player/BP_PlayerCharacter.CoolHook` (`self.As BP Player Character`)))

(fn `UserConstructionScript`)