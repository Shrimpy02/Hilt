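; Holographic platform actor that phases in or out when its create or remove event receives a matching PlatformGroupIndex.
; Tick interpolates emissive and grain opacity on a dynamic material from the construction script, which also shows Mesh1 only while Editing is set.
; Creation unhides the actor and sets collision to Block, then immediately to Ignore.
; Removal hides the actor after a delay, leaving collision untouched.
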(event `CreatePlatform`
  (params (Group :type Integer))
  (if (== Group (`self.PlatformGroupIndex`))
    (`|ExecutionSequence`
      (:`then_0`
        (`self.SetActorHiddenInGame` false)
        (set `self.PhaseIn` true)
        (`PrimitiveComponent.SetCollisionResponseToAllChannels` (`self.Mesh`) "ECR_Block"))
      (:`then_1`
        (set `self.PhaseOut` false)
        (`PrimitiveComponent.SetCollisionResponseToAllChannels` (`self.Mesh`) "ECR_Ignore")))))

(event `RemovePlatform`
  (params (Group :type Integer))
  (if (== Group (`self.PlatformGroupIndex`))
    (`|ExecutionSequence`
      (:`then_0`
        (set `self.PhaseIn` false))
      (:`then_1`
        (set `self.PhaseOut` true)
        (`KismetSystemLibrary.Delay` 3.0)
        (`self.SetActorHiddenInGame` true)))))

(event `self.ReceiveTick`
  (params (DeltaSeconds :type "Float (single-precision)"))
  (bind _material (`self.Material`))
  (bind _material_2 (`self.Material`))
  (bind _material_3 (`self.Material`))
  (bind _material_4 (`self.Material`))
  (`|ExecutionSequence`
    (:`then_0`
      (if (`self.PhaseIn`)
        (`|ExecutionSequence`
          (:`then_0`
            (bind _returnvalue (`MaterialInstanceDynamic.K2_GetScalarParameterValue` _material_2 "Emissive Mod"))
            (`MaterialInstanceDynamic.SetScalarParameterValue` _material_2 "Emissive Mod" (`KismetMathLibrary.FInterpTo` _returnvalue 0.0 (`GameplayStatics.GetWorldDeltaSeconds`) 3.0)))
          (:`then_1`
            (bind _returnvalue_2 (`MaterialInstanceDynamic.K2_GetScalarParameterValue` _material_3 "GrainOpacity"))
            (`MaterialInstanceDynamic.SetScalarParameterValue` _material_3 "GrainOpacity" (`KismetMathLibrary.FInterpTo_Constant` _returnvalue_2 7.0 (`GameplayStatics.GetWorldDeltaSeconds`) 2.0))))))
    (:`then_1`
      (if (`self.PhaseOut`)
        (`|ExecutionSequence`
          (:`then_0`
            (bind _returnvalue_3 (`MaterialInstanceDynamic.K2_GetScalarParameterValue` _material_4 "Emissive Mod"))
            (`MaterialInstanceDynamic.SetScalarParameterValue` _material_4 "Emissive Mod" (`KismetMathLibrary.FInterpTo` _returnvalue_3 100000.0 (`GameplayStatics.GetWorldDeltaSeconds`) 3.0)))
          (:`then_1`
            (bind _returnvalue_4 (`MaterialInstanceDynamic.K2_GetScalarParameterValue` _material "GrainOpacity"))
            (`MaterialInstanceDynamic.SetScalarParameterValue` _material "GrainOpacity" (`KismetMathLibrary.FInterpTo_Constant` _returnvalue_4 0.0 (`GameplayStatics.GetWorldDeltaSeconds`) 4.0))))))))

(fn `UserConstructionScript`
  (`|ExecutionSequence`
    (:`then_0`
      (bind _returnvalue (`PrimitiveComponent.CreateDynamicMaterialInstance` (`self.Mesh`) 0 "/Game/Blueprints/Interactables/Enviroment/Platform/MI_HoloPlatform.MI_HoloPlatform" "None"))
      (set `self.Material` _returnvalue))
    (:`then_1`
      (if (`self.Editing`)
        (`SceneComponent.SetVisibility` (`self.Mesh1`) true false)
        (else
          (`SceneComponent.SetVisibility` (`self.Mesh1`) false false))))))