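; BP_Spinner is an environment actor that rotates continuously.
; Each Tick it adds RotationAdd1 as a local or world rotation, chosen by LocalVsWorld, without scaling by delta time, so spin speed follows frame rate.
; A Sine timeline and location nodes for vertical movement using LocationAdd are present but never run.
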(event `self.ReceiveBeginPlay`)

(event `self.ReceiveTick`
  (params (DeltaSeconds :type "Float (single-precision)"))
  (bind _rotationadd1 (`self.RotationAdd1`))
  (`|ExecutionSequence`
    (:`then_1`
      (if (`self.Local Vs World`)
        (`self.K2_AddActorLocalRotation` _rotationadd1)
        (else
          (`self.K2_AddActorWorldRotation` _rotationadd1))))))

(fn `UserConstructionScript`)