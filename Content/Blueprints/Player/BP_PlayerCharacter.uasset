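; Player character Blueprint that layers feedback onto grappling and handles the pause input.
; Grapple start and stop events toggle hand bone and spark VFX and play end-pose montages, with a freeze, sound and pose for enemy hits.
; Tick prints debug values, feeds velocity to a material parameter collection, speeds up end montages on landing and applies freezes through CustomTimeDilation.
; The construction script sets up the camera arm; the CameraUpdates adjustment is never called.
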(event `CameraUpdates`
  (bind (_cameraarmextratransform_x _cameraarmextratransform_y _cameraarmextratransform_z) (`KismetMathLibrary.BreakVector` (`self.CameraArmExtraTransform`)))
  (bind (_returnvalue_x _returnvalue_y _returnvalue_z) (`KismetMathLibrary.BreakVector` (`SceneComponent.GetForwardVector` (`self.Camera`))))
  (bind (_relativelocation_x _relativelocation_y _relativelocation_z) (`KismetMathLibrary.BreakVector` (`SceneComponent.RelativeLocation` (`self.CameraArm`))))
  ;[0 0.3011 1] Camera Based Events (please Turn in to code later if possible thank you )(Also check construction script)
  (`|ExecutionSequence`
    (:`then_0`
      ;;[1 1 1] Lower Camera While on ground and looking up at hookable object
      (if (and (`self.Is Grappling`) (`NavMovementComponent.IsFalling` (`self.PlayerMovementComponent`)))
        (`|ExecutionSequence`
          (:`then_0`
            (`SceneComponent.K2_SetRelativeLocation` (`self.CameraArm`) (`KismetMathLibrary.VInterpTo` (`KismetMathLibrary.MakeVector` _relativelocation_x _relativelocation_y _relativelocation_z) (`KismetMathLibrary.MakeVector` _relativelocation_x _relativelocation_y _cameraarmextratransform_z) (`GameplayStatics.GetWorldDeltaSeconds`) 5.0) false false :!label _label)))
        (elif (and (> _returnvalue_z 0.5) (`GrapplingComponent.CanGrapple` (`self.GrappleComponent`)))
          (goto _label)
          (else
            (`|ExecutionSequence`
              (:`then_0`
                (`SceneComponent.K2_SetRelativeLocation` (`self.CameraArm`) (`KismetMathLibrary.VInterpTo` (`SceneComponent.RelativeLocation` (`self.CameraArm`)) (`self.CameraArmBaseTransform`) (`GameplayStatics.GetWorldDeltaSeconds`) 5.0) false false)))))))))

(event `self.ReceiveTick`
  (params (DeltaSeconds :type "Float (single-precision)"))
  (bind _score (`ScoreComponent.Score` (`self.ScoreComponent`)))
  ;[0.2137 1 0] Event Tick
  (`|ExecutionSequence`
    (:`then_0`
      ;[1 1 1] Random Debug box?
      (`KismetSystemLibrary.PrintString` (`KismetStringLibrary.Conv_IntToString` (`RocketLauncherComponent.CurrentAmmo` (`self.RocketLauncherComponent`))) true true (struct :`R` 1.0 :`B` 0.764209 :`A` 1.0) 0.0 "1")
      (`KismetSystemLibrary.PrintString` (`KismetStringLibrary.Conv_DoubleToString` (`KismetMathLibrary.VSize` (`self.GetVelocity`))) true true (struct :`R` 1.0 :`G` 0.057227 :`A` 1.0) 0.0 "2"))
    (:`then_1`
      (`KismetSystemLibrary.PrintString` (`KismetStringLibrary.Conv_DoubleToString` _score) true true (make `LinearColor` (`KismetMathLibrary.MapRangeClamped` _score 0.0 5.0 0.0 1.0)) 2.0 "6"))
    (:`then_2`
      (`self.StopPostGrappleMontage`))
    (:`then_3`
      (`self.PostProcessUpdate`))
    (:`then_4`
      (`self.FreezeCheck`))))

(event `CoolHook`
  ;[1 1 1] Delay Effects
  (`|ExecutionSequence`
    (:`then_0`
      (`KismetSystemLibrary.Delay` 0.1)
      (set `self.IsFrozen` true)
      (`GameplayStatics.PlaySound2D` "/Game/Assets/Audio/SFX/Hook/Initial_Blast_wave.Initial_Blast_wave" 1.0 1.0 0.0 null null)
      (`NiagaraFunctionLibrary.SpawnSystemAttached` "/Game/Assets/VFX/GrapplingHook/MiscBonusGrapple/HandShot/NS_GrappleShotHand.NS_GrappleShotHand" (`self.Mesh`) "GrapplingHookSocket" (0.0 0.0 0.0) (struct) "SnapToTargetIncludingScale")
      (`KismetSystemLibrary.Delay` 0.1)
      (set `self.IsFrozen` false))
    (:`then_1`
      (if (> (.z (`GrapplingComponent.GrappleDirection` (`self.GrappleComponent`))) 0.0)
        (`self.PlayAnimMontage` (`KismetArrayLibrary.Array_Random` (`self.Pose Below Anim`)) 1.5)
        (else
          (`self.PlayAnimMontage` (`KismetArrayLibrary.Array_Random` (`self.Pose Above Anim`)) 1.7))))))

(event `PostProcessUpdate`
  (bind _returnvalue (`self.GetVelocity`))
  (bind _returnvalue_2 (`SpringArmComponent.GetTargetRotation` (`self.CameraArm`)))
  (bind _returnvalue_x (`KismetMathLibrary.BreakVector` (* _returnvalue (`KismetMathLibrary.GetForwardVector` _returnvalue_2))))
  (bind (_returnvalue_x_2 _returnvalue_y _returnvalue_z) (`KismetMathLibrary.BreakVector` (* (`self.GetVelocity`) (`KismetMathLibrary.GetUpVector` _returnvalue_2))))
  (bind (_returnvalue_x_3 _returnvalue_y_2) (`KismetMathLibrary.BreakVector` (* (`KismetMathLibrary.GetRightVector` _returnvalue_2) _returnvalue)))
  ;[0 0.3587 1] Post Process Updates
  (`|ExecutionSequence`
    (:`then_0`
      (`KismetMaterialLibrary.SetScalarParameterValue` "/Game/Assets/PostProcessing/MPC_Playerinfluencedmaterials.MPC_Playerinfluencedmaterials" "Speed" (`KismetMathLibrary.MapRangeClamped` (`KismetMathLibrary.VSize` (`self.GetVelocity`)) 0.0 4000.0 0.0 4.0)))
    (:`then_1`
      (`KismetMaterialLibrary.SetVectorParameterValue` "/Game/Assets/PostProcessing/MPC_Playerinfluencedmaterials.MPC_Playerinfluencedmaterials" "FullVelocity" (make `LinearColor` (`KismetMathLibrary.MapRangeClamped` _returnvalue_y_2 -5000.0 5000.0 1.0) (`KismetMathLibrary.MapRangeClamped` _returnvalue_z -6000.0 6000.0 0.0 1.0) (`KismetMathLibrary.MapRangeClamped` _returnvalue_x -1000.0 1000.0 0.0 1.0))))))

(event `KillFreeze`
  ;[1 1 1] KillFreeze
  (set `self.IsFrozen` true)
  (`KismetSystemLibrary.Delay` 2.0)
  (set `self.IsFrozen` false))

(event `FreezeCheck`
  (if (`self.IsFrozen`)
    (set `self.CustomTimeDilation` 0.0)
    (else
      (set `self.CustomTimeDilation` 1.0))))

(event `self.GrappleComponent.OnStartGrapple`
  (params (HitResult :type "HitResult Structure (by ref)"))
  ;[0.3583 1 0] On Start Grapple
  (`|ExecutionSequence`
    (:`then_0`
      (set `self.Is Grappling` true))
    (:`then_1`
      (set `self.GrapplePoint` HitResult_ImpactPoint)
      (set `self.InitalGrappleDirectiom` (`GrapplingComponent.GrappleDirection` (`self.GrappleComponent`))))
    (:`then_2`
      (set `self.IsFrozen` false))
    (:`then_3`
      (`SkinnedMeshComponent.HideBoneByName` (`self.Mesh`) "J_R_Wrist" "PBO_None"))
    (:`then_4`
      (bind _returnvalue (`NiagaraFunctionLibrary.SpawnSystemAttached` "/Game/Assets/VFX/GrapplingHook/MiscBonusGrapple/SpoolReelSparks/NS_SpoolSpark.NS_SpoolSpark" (`self.Mesh`) "SpoolSocket" (0.0 0.0 0.0) (struct) "SnapToTargetIncludingScale"))
      (set `self.SpoolSpark` _returnvalue))
    (:`then_5`
      (if (`self.ActorHasTag` HitResult_HitActor "Enemy")
        (`self.CoolHook`)))))

(event `EnhancedInput|/Game/Blueprints/Player/Input/ActionInputs/IA_PauseButton`
  (params (ActionValue :type Boolean) (ElapsedSeconds :type "Float (double-precision)") (TriggeredSeconds :type "Float (double-precision)") (InputAction :type "InputAction Object Reference" :default "/Game/Blueprints/Player/Input/ActionInputs/IA_PauseButton.IA_PauseButton"))
  ;[1 1 1] Pause Game
  (:`Triggered`
    (bind _asbp_core_hud (cast `/Game/Blueprints/Core/BP_Core_HUD` (`PlayerController.GetHUD` (`GameplayStatics.GetPlayerController` 0))))
    (if (`GameplayStatics.IsGamePaused`)
      (`/Game/Blueprints/Core/BP_Core_HUD.ToggleCoreHUD` _asbp_core_hud)
      (else
        (`/Game/Blueprints/Core/BP_Core_HUD.TogglePause` _asbp_core_hud)))))

(event `self.GrappleComponent.OnStopGrapple`
  (bind _mesh (`self.Mesh`))
  ;[1 0.016 0] GrappleEnd
  (`|ExecutionSequence`
    (:`then_0`
      (set `self.Is Grappling` false))
    (:`then_1`
      (bind _spoolspark (`self.SpoolSpark`)
        (:`then`
          (`ActorComponent.K2_DestroyComponent` _spoolspark))
        (:`else`)))
    (:`then_2`
      (`SkinnedMeshComponent.UnHideBoneByName` (`self.Mesh`) "J_R_Wrist"))
    (:`then_3`
      (`GameplayStatics.PlaySound2D` null 1.0 1.0 0.0 null null))
    (:`then_4`
      (if true
        (if (> (.z (`GrapplingComponent.GrappleDirection` (`self.GrappleComponent`))) 0.0)
          (`|PlayMontage` _mesh (`KismetArrayLibrary.Array_Random` (`self.Pose End Below Anim`))
            (:`then`
              (set `self.PostGrappleMontage` true))
            (:`OnCompleted`
              (set `self.PostGrappleMontage` false :!label _label_2))
            (:`OnInterrupted`
              (goto _label_2)))
          (else
            (`|PlayMontage` _mesh (`KismetArrayLibrary.Array_Random` (`self.Pose End Above Anim`))
              (:`then`
                (set `self.PostGrappleMontage` true))
              (:`OnCompleted`
                (set `self.PostGrappleMontage` false :!label _label_3))
              (:`OnInterrupted`
                (goto _label_3)))))))))

(event `StopPostGrappleMontage`
  (bind _returnvalue (`SkeletalMeshComponent.GetAnimInstance` (`self.Mesh`)))
  ;[1 0.016 0] GrappleEnd
  (if (and (`self.PostGrappleMontage`) (!= (`NavMovementComponent.IsFalling` (`self.CharacterMovement`)) true))
    (`AnimInstance.Montage_SetPlayRate` _returnvalue (`AnimInstance.GetCurrentActiveMontage` _returnvalue) 10.0)))

(fn `UserConstructionScript`
  (`|ExecutionSequence`
    (:`then_0`
      ;[0 0.2738 1] Camera Construction
      (`|ExecutionSequence`
        (:`then_0`
          (set `SpringArmComponent.TargetArmLength` (`self.CameraArmBaseLength`) (`self.CameraArm`)))
        (:`then_1`
          (`SceneComponent.K2_SetRelativeLocation` (`self.CameraArm`) (`self.CameraArmBaseTransform`) false false))))))