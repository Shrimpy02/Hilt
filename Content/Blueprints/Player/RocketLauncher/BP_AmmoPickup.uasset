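; BP_AmmoPickup is a pickup actor that gives the player one round of rocket launcher ammo.
; BeginPlay caches the player character, and overlap on the Pickuprange component increments its RocketLauncherComponent's CurrentAmmo while below ClipSize.
; Any player overlap, even at full ammo, hides the actor for a short delay before showing it again.
; Hiding leaves collision untouched, so the hidden pickup can still grant ammo on a new overlap.
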(event `self.ReceiveBeginPlay`
  (bind _asbp_player_character (cast `/Game/Blueprints/Player/BP_PlayerCharacter` (`GameplayStatics.GetPlayerCharacter` 0)))
  (set `self.Player` _asbp_player_character))

(event `self.Pickuprange.OnComponentBeginOverlap`
  (params (OverlappedComponent :type "PrimitiveComponent Object Reference") (OtherActor :type "Actor Object Reference") (OtherComp :type "PrimitiveComponent Object Reference") (OtherBodyIndex :type Integer) (bFromSweep :type Boolean) (SweepResult :type "HitResult Structure (by ref)"))
  (bind _rocketlaunchercomponent (`PlayerCharacter.RocketLauncherComponent` (`self.Player`)))
  (bind _rocketlaunchercomponent_2 (`PlayerCharacter.RocketLauncherComponent` (`self.Player`)))
  (if (== OtherActor (`self.Player`))
    (`|ExecutionSequence`
      (:`then_0`
        (if (< (`RocketLauncherComponent.CurrentAmmo` _rocketlaunchercomponent) (`RocketLauncherComponent.ClipSize` _rocketlaunchercomponent))
          (set `RocketLauncherComponent.CurrentAmmo` (+ (`RocketLauncherComponent.CurrentAmmo` _rocketlaunchercomponent_2) 1) _rocketlaunchercomponent_2)))
      (:`then_1`
        (`self.SetActorHiddenInGame` true)
        (`KismetSystemLibrary.Delay` 2.0)
        (`self.SetActorHiddenInGame` false)))))

(fn `UserConstructionScript`)