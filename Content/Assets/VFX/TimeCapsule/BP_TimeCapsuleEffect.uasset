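; Time capsule VFX Blueprint that puts six temporary trail effects on the player character that owns it.
; On BeginPlay it casts its owner to BP_PlayerCharacter and snaps the left and right trail components to matching TrailSlot sockets on the character mesh, keeping world scale.
; After a short fixed delay it destroys the trail components, but does not destroy itself.
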(event `self.ReceiveBeginPlay`
  (`|ExecutionSequence`
    (:`then_0`
      (bind _asbp_player_character (cast `/Game/Blueprints/Player/BP_PlayerCharacter` (`self.GetOwner`)))
      (set `self.As BP Player Character` _asbp_player_character)
      (`|ExecutionSequence`
        (:`then_0`
          (bind _mesh (`Character.Mesh` _asbp_player_character))
          (`SceneComponent.K2_AttachToComponent` (`self.LS_Trail`) _mesh "L_S_TrailSlot" "SnapToTarget" "SnapToTarget" "KeepWorld" true))
        (:`then_1`
          (`SceneComponent.K2_AttachToComponent` (`self.LH_Trail`) _mesh "L_H_TrailSlot" "SnapToTarget" "SnapToTarget" "KeepWorld" true))
        (:`then_2`
          (`SceneComponent.K2_AttachToComponent` (`self.LF_Trail`) _mesh "L_F_TrailSlot" "SnapToTarget" "SnapToTarget" "KeepWorld" true))
        (:`then_3`
          (`SceneComponent.K2_AttachToComponent` (`self.RS_Trail`) _mesh "R_S_TrailSlot" "SnapToTarget" "SnapToTarget" "KeepWorld" true))
        (:`then_4`
          (`SceneComponent.K2_AttachToComponent` (`self.RH_Trail`) _mesh "R_H_TrailSlot" "SnapToTarget" "SnapToTarget" "KeepWorld" true))
        (:`then_5`
          (`SceneComponent.K2_AttachToComponent` (`self.RF_Trail`) _mesh "R_F_TrailSlot" "SnapToTarget" "SnapToTarget" "KeepWorld" true))))
    (:`then_1`
      (`KismetSystemLibrary.Delay` 2.0)
      (for _array_element (`|MakeArray` (`self.RF_Trail`) (`self.RH_Trail`) (`self.LH_Trail`) (`self.RS_Trail`) (`self.LS_Trail`) (`self.LF_Trail`))
        (`ActorComponent.K2_DestroyComponent` _array_element)))))

(fn `UserConstructionScript`)